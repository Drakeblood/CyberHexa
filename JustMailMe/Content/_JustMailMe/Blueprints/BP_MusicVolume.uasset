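; VR grabbable knob actor that controls the volume of an ambient sound, likely music given the asset name.
; Grabbing starts a fast looping timer that copies the motion controller's world roll onto the knob mesh (Przekretlo), keeping its pitch and yaw.
; The same roll is range-mapped, clamped, to the AmbientSound volume multiplier.
; Dropping clears the controller reference and requests a timer pause by function name.
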(event OnGrabbed(GrabComponent)
  (params (motionController :type Motion%20Controller%20Component%20Object%20Reference))
  (Variables|Default|SetMotion%20Controller motionController)
  (bind _returnvalue (Utilities|Time|SetTimerbyEvent (delegate Custom|UpdateRotation) 0.02 true true)))

(event OnDropped(GrabComponent)
  (Variables|Default|SetMotion%20Controller 0)
  (Class|KismetSystemLibrary|PauseTimer 0 "UpdateRotation"))

(event Custom|UpdateRotation
  (bind _przekretlo (Variables|Default|Getprzekretlo))
  (bind _returnvalue (Transformation|GetWorldRotation _przekretlo))
  (Variables|Default|SetCurrentRotation (Transformation|GetWorldRotation (Variables|Default|GetMotion%20Controller)))
  (Transformation|SetWorldRotation _przekretlo (Math|Rotator|MakeRotator (.roll (Variables|Default|GetCurrentRotation)) (.pitch _returnvalue) (.yaw _returnvalue)) false false)
  (Audio|Components|Audio|SetVolumeMultiplier (Variables|/Script/Engine.AmbientSound|GetAudioComponent (Variables|Default|GetambientSound)) (Math|Float|MapRangeClamped (.roll (Variables|Default|GetCurrentRotation)) 5e+01 -5e+01 0.0 1.5) :!class /Script/Engine.AudioComponent))

(event EventBeginPlay)

(event Collision|EventActorBeginOverlap
  (params (OtherActor :type Actor%20Object%20Reference)))

(event EventTick
  (params (DeltaSeconds :type Float%20%28single-precision%29)))

(fn ConstructionScript)