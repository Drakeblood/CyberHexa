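; Cursor tracer actor that acts as a movable cursor, carrying a widget interaction reference.
; AddMovementVector moves it with a sweep along its own right and up vectors, scaled by MovementScale, then fires LocationChanged with WidgetInteraction.
; The construction script records the starting X location in InitialX, which the graphs shown never read; BeginPlay, overlap and Tick are disabled stubs.
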(event Custom|AddMovementVector
  (params (X :type Float%20%28double-precision%29) (Y :type Float%20%28double-precision%29))
  (Transformation|SetActorLocation (+ (Transformation|GetActorLocation) (* (Transformation|GetActorRightVector) X (Variables|Default|GetMovementScale)) (* (Transformation|GetActorUpVector) Y (Variables|Default|GetMovementScale))) true false)
  (Default|CallLocationChanged (Variables|Default|GetWidgetInteraction)))

(event EventBeginPlay)

(event Collision|EventActorBeginOverlap
  (params (OtherActor :type Actor%20Object%20Reference)))

(event EventTick
  (params (DeltaSeconds :type Float%20%28single-precision%29)))

(fn ConstructionScript
  (Variables|Default|SetInitialX (.x (Transformation|GetActorLocation))))