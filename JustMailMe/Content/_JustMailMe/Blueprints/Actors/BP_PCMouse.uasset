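; BP_PCMouse is a physical computer mouse actor whose movement in the world drives the cursor of a linked Computer.
; Each Tick it measures how far the actor moved since the previous tick and ignores near-zero deltas.
; While MouseWorkingArea overlaps any BP_PCMouse, it passes the delta to the Computer's CursorTracer, swapping world X and Y to get cursor axes.
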(event EventTick
  (params (DeltaSeconds :type Float%20%28single-precision%29))
  (Utilities|FlowControl|Sequence
    (:then_0
      (Variables|Default|SetCurrentDelta (- (Transformation|GetActorLocation) (Variables|Default|GetPreviousTickLocation)))
      (if (not (Math|Vector|VectorIsNearlyZero (Variables|Default|GetCurrentDelta)))
        (if (Math|Conversions|ToBoolean(Integer) (Utilities|Array|Length (Collision|GetOverlappingActors (Variables|Default|GetMouseWorkingArea) "BP_PCMouse_C" :!class /Script/Engine.Actor)))
          (Default|AddMovementVector (Variables|/Game/_JustMailMe/Blueprints/Actors/BP_Computer3D.BP_Computer3D_C|GetCursorTracer (Variables|Default|GetComputer)) (.y (Variables|Default|GetCurrentDelta)) (.x (Variables|Default|GetCurrentDelta))))))
    (:then_1
      (Variables|Default|SetPreviousTickLocation (Transformation|GetActorLocation)))))

(event EventBeginPlay
  (Variables|Default|SetPreviousTickLocation (Transformation|GetActorLocation)))

(fn ConstructionScript)