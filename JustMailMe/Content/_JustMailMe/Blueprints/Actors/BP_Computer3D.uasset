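; Clickable 3D computer actor that opens the monitor screen UI for the player.
; On BeginPlay it caches its child cursor tracer, registers itself with VRGameMode and binds click and hover events.
; A click sets the camera pawn's Monitor flag, waits briefly, then creates WBP_Monitor or reactivates the existing one.
; Hover and ChangeMaterial events are empty, with their visibility and material nodes left disconnected.
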(event Custom|OnClicked_Event
  (params (TouchedActor :type Actor%20Object%20Reference) (ButtonPressed :type Key%20Structure :default "None"))
  (Variables|/Game/_CyberHexa/Blueprints/BP_CameraPawn.BP_CameraPawn_C|SetMonitor (CallFunction|GetCameraPawn) true)
  (Utilities|FlowControl|Delay 0.5)
  (bind _monitorwidget (Variables|Default|GetMonitorWidget)
    (:then
      (CallFunction|ActivateWidget _monitorwidget))
    (:else
      (Variables|Default|SetMonitorWidget (.AsWBP%20Monitor (Utilities|Casting|CastToWBP_Monitor (CallFunction|GetWidget "/Game/_CyberHexa/Blueprints/Widgets/WBP_Monitor.WBP_Monitor_C" true)))))))

(event Custom|ChangeMaterial
  (params (Material :type Material%20Interface%20Object%20Reference)))

(event Custom|OnBeginCursorOver_Event
  (params (TouchedActor :type Actor%20Object%20Reference)))

(event Custom|OnEndCursorOver_Event
  (params (TouchedActor :type Actor%20Object%20Reference)))

(event EventBeginPlay
  (Variables|Default|SetCursorTracer (.AsBP%20Cursor%20Tracer (Utilities|Casting|CastToBP_CursorTracer (Variables|/Script/Engine.ChildActorComponent|GetChildActor (Variables|Default|GetChildActor)))))
  (Variables|/Game/VRTemplate/Blueprints/VRGameMode.VRGameMode_C|SetComputer3D (.AsVRGame%20Mode (Utilities|Casting|CastToVRGameMode (Game|GetGameMode))) self)
  (EventDispatchers|BindEventtoOnClicked (EventDispatchers|CreateEvent :!event Custom|OnClicked_Event))
  (EventDispatchers|BindEventtoOnBeginCursorOver (EventDispatchers|CreateEvent :!event Custom|OnBeginCursorOver_Event))
  (EventDispatchers|BindEventtoOnEndCursorOver (EventDispatchers|CreateEvent :!event Custom|OnEndCursorOver_Event)))

(fn ConstructionScript)