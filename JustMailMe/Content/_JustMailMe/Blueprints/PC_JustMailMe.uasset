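; Player controller for JustMailMe that provides debug controls for testing the PC mouse, button, power switch and 3D monitor without normal interaction.
; Held keys nudge BP_PCMouse or scroll the game mode's Monitor3D every frame through Gate and DelayUntilNextTick loops.
; Other keys fake button overlaps and call the mouse's input test.
; Separate functions debug-press BP_Wlancznik and trigger VRGameMode error, ad, fake-mail and video-ad glitches.
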(event Input|KeyboardEvents|DebugKeyB
  (params (Key :type Key%20Structure :default "None") (ActionValue :type Input%20Action%20Value%20Structure))
  (:Pressed
    (bind _returnvalue (Actor|GetActorOfClass "/Game/_CyberHexa/Blueprints/BP_Button.BP_Button_C"))
    (Default|TestStartOverlap _returnvalue))
  (:Released
    (bind _returnvalue_2 (Actor|GetActorOfClass "/Game/_CyberHexa/Blueprints/BP_Button.BP_Button_C"))
    (Default|TestEndOverlap _returnvalue_2)))

(event Input|KeyboardEvents|DebugKeyRight
  (params (Key :type Key%20Structure :default "None") (ActionValue :type Input%20Action%20Value%20Structure))
  (:Pressed
    (Utilities|FlowControl|Sequence
      (:then_0
        (goto _label Open))
      (:then_1
        (Utilities|FlowControl|Gate true :!label _label
          (:Exit
            (bind _returnvalue (Actor|GetActorOfClass "/Game/_JustMailMe/Blueprints/Actors/BP_PCMouse.BP_PCMouse_C"))
            (Transformation|AddActorLocalOffset _returnvalue (Math|Vector|MakeVector 0.0 -0.2 0.0) false false)
            (Utilities|FlowControl|DelayUntilNextTick)
            (goto _label))))))
  (:Released
    (goto _label Close)))

(event Input|KeyboardEvents|DebugKeyLeft
  (params (Key :type Key%20Structure :default "None") (ActionValue :type Input%20Action%20Value%20Structure))
  (:Pressed
    (Utilities|FlowControl|Sequence
      (:then_0
        (goto _label Open))
      (:then_1
        (Utilities|FlowControl|Gate true :!label _label
          (:Exit
            (bind _returnvalue (Actor|GetActorOfClass "/Game/_JustMailMe/Blueprints/Actors/BP_PCMouse.BP_PCMouse_C"))
            (Transformation|AddActorLocalOffset _returnvalue (Math|Vector|MakeVector 0.0 0.2 0.0) false false)
            (Utilities|FlowControl|DelayUntilNextTick)
            (goto _label))))))
  (:Released
    (goto _label Close)))

(event Input|KeyboardEvents|DebugKeyUp
  (params (Key :type Key%20Structure :default "None") (ActionValue :type Input%20Action%20Value%20Structure))
  (:Pressed
    (Utilities|FlowControl|Sequence
      (:then_0
        (goto _label Open))
      (:then_1
        (Utilities|FlowControl|Gate true :!label _label
          (:Exit
            (bind _returnvalue (Actor|GetActorOfClass "/Game/_JustMailMe/Blueprints/Actors/BP_PCMouse.BP_PCMouse_C"))
            (Transformation|AddActorLocalOffset _returnvalue (Math|Vector|MakeVector -0.2 0.0 0.0) false false)
            (Utilities|FlowControl|DelayUntilNextTick)
            (goto _label))))))
  (:Released
    (goto _label Close)))

(event Input|KeyboardEvents|DebugKeyDown
  (params (Key :type Key%20Structure :default "None") (ActionValue :type Input%20Action%20Value%20Structure))
  (:Pressed
    (Utilities|FlowControl|Sequence
      (:then_0
        (goto _label Open))
      (:then_1
        (Utilities|FlowControl|Gate true :!label _label
          (:Exit
            (bind _returnvalue (Actor|GetActorOfClass "/Game/_JustMailMe/Blueprints/Actors/BP_PCMouse.BP_PCMouse_C"))
            (Transformation|AddActorLocalOffset _returnvalue (Math|Vector|MakeVector 0.2 0.0 0.0) false false)
            (Utilities|FlowControl|DelayUntilNextTick)
            (goto _label))))))
  (:Released
    (goto _label Close)))

(event Input|KeyboardEvents|DebugKeyG
  (params (Key :type Key%20Structure :default "None") (ActionValue :type Input%20Action%20Value%20Structure))
  (:Pressed
    (bind _returnvalue (Actor|GetActorOfClass "/Game/_JustMailMe/Blueprints/Actors/BP_PCMouse.BP_PCMouse_C"))
    (Default|TestEnableInput _returnvalue)))

(event Input|KeyboardEvents|DebugKeyI
  (params (Key :type Key%20Structure :default "None") (ActionValue :type Input%20Action%20Value%20Structure))
  (:Pressed
    (Utilities|FlowControl|Sequence
      (:then_0
        (goto _label Open))
      (:then_1
        (Utilities|Gate true :!label _label
          (:Exit
            (Default|AddScrollInput (Variables|/Game/VRTemplate/Blueprints/VRGameMode.VRGameMode_C|GetMonitor3D (.AsVRGame%20Mode (Utilities|Casting|CastToVRGameMode (Game|GetGameMode)))) -1.0)
            (Utilities|FlowControl|DelayUntilNextTick)
            (goto _label))))))
  (:Released
    (goto _label Close)))

(event Input|KeyboardEvents|DebugKeyK
  (params (Key :type Key%20Structure :default "None") (ActionValue :type Input%20Action%20Value%20Structure))
  (:Pressed
    (Utilities|FlowControl|Sequence
      (:then_0
        (goto _label Open))
      (:then_1
        (Utilities|Gate true :!label _label
          (:Exit
            (Default|AddScrollInput (Variables|/Game/VRTemplate/Blueprints/VRGameMode.VRGameMode_C|GetMonitor3D (.AsVRGame%20Mode (Utilities|Casting|CastToVRGameMode (Game|GetGameMode)))) 1.0)
            (Utilities|FlowControl|DelayUntilNextTick)
            (goto _label))))))
  (:Released
    (goto _label Close)))

(fn ConstructionScript)

(fn PressWlacznik
  (bind _returnvalue (Actor|GetActorOfClass "/Game/_CyberHexa/Blueprints/BP_Wlancznik.BP_Wlancznik_C"))
  (Default|DebugPress _returnvalue))

(fn AddBladMachen
  (bind _asvrgame_mode (Utilities|Casting|CastToVRGameMode (Game|GetGameMode)))
  (Default|AddBladMachen _asvrgame_mode))

(fn AddGlitchReklama
  (bind _asvrgame_mode (Utilities|Casting|CastToVRGameMode (Game|GetGameMode)))
  (Default|GlitchReklama _asvrgame_mode))

(fn AddGlitchFakeMail
  (bind _asvrgame_mode (Utilities|Casting|CastToVRGameMode (Game|GetGameMode)))
  (Default|GlitchFakeMail _asvrgame_mode))

(fn AddGlitchReklamaVideo
  (bind _asvrgame_mode (Utilities|Casting|CastToVRGameMode (Game|GetGameMode)))
  (Default|GlitchReklamaVideo _asvrgame_mode))