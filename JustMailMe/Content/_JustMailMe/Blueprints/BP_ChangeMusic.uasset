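; BP_ChangeMusic is an in-world music switcher that changes the track on a referenced AmbientSound when an actor tagged "player" enters one of its two triggers.
; The BaseJazz trigger restores the jazz background track, while the Songs trigger advances a wrapping index through the Musics array.
; Each switch plays a click sound and lowers the volume multiplier, with a DoOnce per trigger that resets when the player leaves.
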(event OnComponentBeginOverlap(baseJazz)
  (params (OverlappedComponent :type Primitive%20Component%20Object%20Reference) (OtherActor :type Actor%20Object%20Reference) (OtherComp :type Primitive%20Component%20Object%20Reference) (OtherBodyIndex :type Integer) (bFromSweep :type Boolean) (SweepResult :type Hit%20Result%20Structure%20%28by%20ref%29))
  (bind _ambient_sound (Variables|Default|Getambient\Sound))
  (bind _audiocomponent (Variables|/Script/Engine.AmbientSound|GetAudioComponent _ambient_sound))
  (if (Actor|ActorHasTag OtherActor "player")
    (Utilities|FlowControl|DoOnce false
      (:Completed
        (Audio|PlaySoundatLocation "/Game/VRTemplate/Audio/click_computer.click_computer" (Transformation|GetActorLocation) "0, 0, 0" 1.0 1.0 0.0 0 0 0 0)
        (Audio|Components|Audio|SetSound _audiocomponent "/Game/VRTemplate/Audio/jazz-background-music-353636.jazz-background-music-353636")
        (Audio|Components|Audio|SetVolumeMultiplier _audiocomponent 0.2 :!class /Script/Engine.AudioComponent)))))

(event OnComponentEndOverlap(baseJazz)
  (params (OverlappedComponent :type Primitive%20Component%20Object%20Reference) (OtherActor :type Actor%20Object%20Reference) (OtherComp :type Primitive%20Component%20Object%20Reference) (OtherBodyIndex :type Integer))
  (bind _ambient_sound (Variables|Default|Getambient\Sound))
  (bind _audiocomponent (Variables|/Script/Engine.AmbientSound|GetAudioComponent _ambient_sound))
  (if (Actor|ActorHasTag OtherActor "player")
    (Utilities|FlowControl|DoOnce false) ; enters at Reset
  ))

(event OnComponentBeginOverlap(songs)
  (params (OverlappedComponent :type Primitive%20Component%20Object%20Reference) (OtherActor :type Actor%20Object%20Reference) (OtherComp :type Primitive%20Component%20Object%20Reference) (OtherBodyIndex :type Integer) (bFromSweep :type Boolean) (SweepResult :type Hit%20Result%20Structure%20%28by%20ref%29))
  (bind _ambient_sound (Variables|Default|Getambient\Sound))
  (bind _audiocomponent (Variables|/Script/Engine.AmbientSound|GetAudioComponent _ambient_sound))
  (if (Actor|ActorHasTag OtherActor "player")
    (Utilities|FlowControl|DoOnce false
      (:Completed
        (Audio|PlaySoundatLocation "/Game/VRTemplate/Audio/click_computer.click_computer" (Transformation|GetActorLocation) "0, 0, 0" 1.0 1.0 0.0 0 0 0 0)
        (Utilities|IncrementInt (Variables|Default|GetMusicIndex)
          (:%20%20
            (if (> (Variables|Default|GetMusicIndex) 2)
              (Variables|Default|SetMusicIndex 0))
            (Audio|Components|Audio|SetSound _audiocomponent (Utilities|Array|Get(acopy) (Variables|Default|GetMusics) (Variables|Default|GetMusicIndex)))
            (Audio|Components|Audio|SetVolumeMultiplier _audiocomponent 0.2 :!class /Script/Engine.AudioComponent)))))))

(event OnComponentEndOverlap(songs)
  (params (OverlappedComponent :type Primitive%20Component%20Object%20Reference) (OtherActor :type Actor%20Object%20Reference) (OtherComp :type Primitive%20Component%20Object%20Reference) (OtherBodyIndex :type Integer))
  (bind _ambient_sound (Variables|Default|Getambient\Sound))
  (bind _audiocomponent (Variables|/Script/Engine.AmbientSound|GetAudioComponent _ambient_sound))
  (if (Actor|ActorHasTag OtherActor "player")
    (Utilities|FlowControl|DoOnce false) ; enters at Reset
  ))

(event EventBeginPlay)

(event Collision|EventActorBeginOverlap
  (params (OtherActor :type Actor%20Object%20Reference)))

(event EventTick
  (params (DeltaSeconds :type Float%20%28single-precision%29)))

(fn ConstructionScript)