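; BP_Kartka is a paper sheet prop that highlights when the player is near and can be grabbed.
; Box overlaps with actors tagged "player" toggle the Plane's "Emmision" material parameter, and dropping through GrabComponent enables physics on the Plane.
; The construction script applies the Material variable to the Plane.
; Older click, cursor-hover and socket-attach logic is left disconnected, and several events are empty.
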(event OnComponentBeginOverlap(Box)
  (params (OverlappedComponent :type Primitive%20Component%20Object%20Reference) (OtherActor :type Actor%20Object%20Reference) (OtherComp :type Primitive%20Component%20Object%20Reference) (OtherBodyIndex :type Integer) (bFromSweep :type Boolean) (SweepResult :type Hit%20Result%20Structure%20%28by%20ref%29))
  (if (Actor|ActorHasTag OtherActor "player")
    (Rendering|Material|SetScalarParameterValueonMaterials (Variables|Default|GetPlane) "Emmision" 1e+01)))

(event OnComponentEndOverlap(Box)
  (params (OverlappedComponent :type Primitive%20Component%20Object%20Reference) (OtherActor :type Actor%20Object%20Reference) (OtherComp :type Primitive%20Component%20Object%20Reference) (OtherBodyIndex :type Integer))
  (if (Actor|ActorHasTag OtherActor "player")
    (Rendering|Material|SetScalarParameterValueonMaterials (Variables|Default|GetPlane) "Emmision" 0.0)))

(event OnDropped(GrabComponent)
  (Physics|SetSimulatePhysics (Variables|Default|GetPlane) true))

(event Custom|OnClicked_Event
  (params (TouchedActor :type Actor%20Object%20Reference) (ButtonPressed :type Key%20Structure :default "None")))

(event Custom|OnBeginCursorOver_Event
  (params (TouchedActor :type Actor%20Object%20Reference)))

(event Custom|OnEndCursorOver_Event
  (params (TouchedActor :type Actor%20Object%20Reference))
  (Rendering|Material|SetScalarParameterValueonMaterials (Variables|Default|GetPlane) "Emmision" 0.0))

(event EventBeginPlay)

(event EventAddKartka)

(fn ConstructionScript
  (Rendering|Material|SetMaterial (Variables|Default|GetPlane) 0 (Variables|Default|GetMaterial)))