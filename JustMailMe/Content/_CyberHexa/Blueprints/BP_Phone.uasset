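; BP_Phone is a grabbable phone that rings by wobbling on a looping timeline until picked up, delivering timed text messages.
; Grabbing shows one text on the first call and another afterwards on a TextRender, while a player-tagged overlap makes the mesh glow.
; Dropping it schedules the next ring after a delay, and the first drop also spawns a physics BP_Kartka.
; An older click-driven WBP_PhoneCall widget path remains disconnected.
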(event OnGrabbed(GrabComponent)
  (bind _textrender (Variables|Default|GetTextRender))
  (bind _textrender_2 (Variables|Default|GetTextRender))
  (Variables|Default|SetClick true)
  (if (Variables|Default|GetFirstCall)
    (Utilities|FlowControl|Delay 1.0)
    (Rendering|SetVisibility _textrender_2 true false)
    (Rendering|Components|TextRender|SetText (Variables|Default|GetTextRender) (Variables|Default|GetFirstText))
    (Utilities|FlowControl|Delay 1e+01)
    (Rendering|SetVisibility _textrender_2 false false)
    (else
      (Utilities|FlowControl|Delay 1.0)
      (Rendering|SetVisibility _textrender true false)
      (Rendering|Components|TextRender|SetText (Variables|Default|GetTextRender) (Variables|Default|GetUgaBuga))
      (Utilities|FlowControl|Delay 1e+01)
      (Rendering|SetVisibility _textrender false false))))

(event OnDropped(GrabComponent)
  (if (Variables|Default|GetFirstCall)
    (bind _returnvalue (Game|SpawnActorfromClass "/Game/_CyberHexa/Papiery/BP_Kartka.BP_Kartka_C" (Math|Transform|MakeTransform "504.860423,-184.999031,567.827387" "0.000000,-66.193350,0.000000" "0.200000,0.200000,0.200000") "Undefined" "MultiplyWithRoot" 0 0))
    (Physics|SetSimulatePhysics (Variables|/Game/_CyberHexa/Papiery/BP_Kartka.BP_Kartka_C|GetPlane _returnvalue) true)
    (CallFunction|PhantomCall)
    (Variables|Default|SetFirstCall false)
    (else
      (CallFunction|PhantomCall))))

(event OnComponentBeginOverlap(Box)
  (params (OverlappedComponent :type Primitive%20Component%20Object%20Reference) (OtherActor :type Actor%20Object%20Reference) (OtherComp :type Primitive%20Component%20Object%20Reference) (OtherBodyIndex :type Integer) (bFromSweep :type Boolean) (SweepResult :type Hit%20Result%20Structure%20%28by%20ref%29))
  (if (Actor|ActorHasTag OtherActor "player")
    (Rendering|Material|SetScalarParameterValueonMaterials (Variables|Default|GetStaticMesh) "Emmision" 1e+01)))

(event OnComponentEndOverlap(Box)
  (params (OverlappedComponent :type Primitive%20Component%20Object%20Reference) (OtherActor :type Actor%20Object%20Reference) (OtherComp :type Primitive%20Component%20Object%20Reference) (OtherBodyIndex :type Integer))
  (if (Actor|ActorHasTag OtherActor "player")
    (Rendering|Material|SetScalarParameterValueonMaterials (Variables|Default|GetStaticMesh) "Emmision" 0.0)))

(event Custom|OnClicked_Event
  (params (TouchedActor :type Actor%20Object%20Reference) (ButtonPressed :type Key%20Structure :default "None")))

(event Custom|OnTextsEnd_Event
  (Variables|/Game/_CyberHexa/Blueprints/BP_CameraPawn.BP_CameraPawn_C|SetPhone (CallFunction|GetCameraPawn) false)
  (Utilities|FlowControl|Delay 0.55)
  (Transformation|DetachFromComponent (Variables|Default|GetStaticMesh) "KeepWorld" "KeepWorld" "KeepWorld" true)
  (Utilities|FlowControl|Delay (Math|Random|RandomFloatinRange 2.0 5.0))
  (Default|GotoRoom (CallFunction|GetSplinePath)))

(event Custom|OnBeginCursorOver_Event
  (params (TouchedActor :type Actor%20Object%20Reference)))

(event Custom|OnEndCursorOver_Event
  (params (TouchedActor :type Actor%20Object%20Reference)))

(event Custom|Ringing
  (bind _newtrack_0 (Timeline|Timeline Play)
    (:Update
      (Transformation|SetActorRotation (Math|Rotator|MakeRotator (* _newtrack_0 5.0) (* _newtrack_0 1e+01) 0.0)))
    (:Finished
      (Utilities|FlowControl|Delay 1.0)
      (if (not (Variables|Default|GetClick))
        (Utilities|FlowControl|FlipFlop
          (:A
            (Timeline|Timeline ReverseFromEnd))
          (:B
            (Timeline|Timeline PlayFromStart)))))))

(event Custom|PhantomCall
  (if (Variables|Default|GetFirstCall)
    (Utilities|FlowControl|Delay 5e+01)
    (else
      (Utilities|FlowControl|Delay (Math|Random|RandomFloatinRange 3e+01 6e+01))))
  (Variables|Default|SetClick false)
  (CallFunction|Ringing))

(event EventBeginPlay
  (CallFunction|Ringing))

(fn ConstructionScript)