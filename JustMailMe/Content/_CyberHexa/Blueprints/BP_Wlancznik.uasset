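; BP_Wlancznik is a computer power switch that the player toggles by overlapping its box, with a debug event as an alternate trigger.
; A DoOnce and FlipFlop alternate power-on, showing a loading material on a screen plane before hiding it, and power-off, showing black.
; Each branch notifies VRGameMode to check glitches or shut down, and re-arms after a two-second delay.
; A separate Bluescreen event displays the blue-screen material.
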(event OnComponentBeginOverlap(Box)
  (params (OverlappedComponent :type Primitive%20Component%20Object%20Reference) (OtherActor :type Actor%20Object%20Reference) (OtherComp :type Primitive%20Component%20Object%20Reference) (OtherBodyIndex :type Integer) (bFromSweep :type Boolean) (SweepResult :type Hit%20Result%20Structure%20%28by%20ref%29))
  (bind _returnvalue (Game|GetGameMode))
  (bind _asvrgame_mode (Utilities|Casting|CastToVRGameMode _returnvalue))
  (if (Actor|ActorHasTag OtherActor "player")
    (Utilities|FlowControl|DoOnce false :!label _label
      (:Completed
        (Utilities|FlipFlop
          (:A
            (Rendering|Material|SetMaterial (Variables|Default|GetPlane) 0 "/Game/_CyberHexa/UI/Pulpit/M_LoadingScreen.M_LoadingScreen")
            (Utilities|FlowControl|Delay 2.0)
            (Rendering|SetVisibility (Variables|Default|GetPlane) false false)
            (Default|CheckGlitchesAfterComputerPoweron _asvrgame_mode)
            (goto _label Reset))
          (:B
            (Rendering|Material|SetMaterial (Variables|Default|GetPlane) 0 "/Game/_CyberHexa/Blueprints/M_BlackScreen.M_BlackScreen")
            (Rendering|SetVisibility (Variables|Default|GetPlane) true false)
            (Default|ShutdownComputer _asvrgame_mode)
            (Utilities|FlowControl|Delay 2.0)
            (goto _label Reset)))))))

(event OnComponentEndOverlap(Box)
  (params (OverlappedComponent :type Primitive%20Component%20Object%20Reference) (OtherActor :type Actor%20Object%20Reference) (OtherComp :type Primitive%20Component%20Object%20Reference) (OtherBodyIndex :type Integer))
  (if (Actor|ActorHasTag (stale OnComponentBeginOverlap(Box) OtherActor) "player")
    _))

(event Custom|DebugPress
  (bind _returnvalue (Game|GetGameMode))
  (bind _asvrgame_mode (Utilities|Casting|CastToVRGameMode _returnvalue))
  (Utilities|FlowControl|DoOnce false :!label _label
    (:Completed
      (Utilities|FlipFlop
        (:A
          (Rendering|Material|SetMaterial (Variables|Default|GetPlane) 0 "/Game/_CyberHexa/UI/Pulpit/M_LoadingScreen.M_LoadingScreen")
          (Utilities|FlowControl|Delay 2.0)
          (Rendering|SetVisibility (Variables|Default|GetPlane) false false)
          (Default|CheckGlitchesAfterComputerPoweron _asvrgame_mode)
          (goto _label Reset))
        (:B
          (Rendering|Material|SetMaterial (Variables|Default|GetPlane) 0 "/Game/_CyberHexa/Blueprints/M_BlackScreen.M_BlackScreen")
          (Rendering|SetVisibility (Variables|Default|GetPlane) true false)
          (Default|ShutdownComputer _asvrgame_mode)
          (Utilities|FlowControl|Delay 2.0)
          (goto _label Reset))))))

(event Custom|Bluescreen
  (Rendering|Material|SetMaterial (Variables|Default|GetPlane) 0 "/Game/_CyberHexa/UI/Pulpit/M_BlueScreen.M_BlueScreen")
  (Rendering|SetVisibility (Variables|Default|GetPlane) true false))

(event EventBeginPlay)

(event Collision|EventActorBeginOverlap
  (params (OtherActor :type Actor%20Object%20Reference)))

(event EventTick
  (params (DeltaSeconds :type Float%20%28single-precision%29)))

(fn ConstructionScript)