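; Scripted NPC visitor Bobik who follows a spline into a room to offer his CV, then leaves.
; GoToRoom and ExitRoom move the capsule by re-calling themselves each tick; GoToRoom stops at spline point 3 for WBP_PhoneCall dialogue with a hand-over montage.
; Text end triggers the exit and a delayed job-application email to WBP_Monitor; hits from "throw"-tagged actors also trigger the exit.
; Hover glow, click binding and paper-spawning logic are disconnected.
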(event OnComponentHit(Capsule)
  (params (HitComponent :type Primitive%20Component%20Object%20Reference) (OtherActor :type Actor%20Object%20Reference) (OtherComp :type Primitive%20Component%20Object%20Reference) (NormalImpulse :type Vector :default "0, 0, 0") (Hit :type Hit%20Result%20Structure%20%28by%20ref%29))
  (if (Actor|ActorHasTag OtherActor "throw")
    (CallFunction|ExitRoom)))

(event Custom|GoToRoom
  (bind _userwidget (CallFunction|GetWidget "/Game/_CyberHexa/Blueprints/Widgets/WBP_PhoneCall.WBP_PhoneCall_C" true))
  (bind _aswbp_phone_call (Utilities|Casting|CastToWBP_PhoneCall _userwidget))
  (Variables|Default|SetMove true)
  (bind _output_get (Variables|Default|SetDistanceAlongSpline (+ (* (Utilities|Time|GetWorldDeltaSeconds) (Variables|Default|GetSplineSpeed)) (Variables|Default|GetDistanceAlongSpline))))
  (if (> _output_get (Spline|GetDistanceAlongSplineatSplinePoint (Variables|Default|GetSpline) 3))
    (Variables|Default|SetMove false)
    (Default|SetTextsandStart _aswbp_phone_call (Utilities|Array|MakeArray "Here is my CV." "You should send your CV via our standardised system. Just mail me!"))
    (Variables|Default|SetTalking true)
    (EventDispatchers|AssignOnNextText _aswbp_phone_call (delegate Custom|OnNextText_Event))
    (else
      (Transformation|SetRelativeTransform (Variables|Default|GetCapsule) (Math|Transform|MakeTransform (Math|Vector|MakeVector (.x (.location (Spline|GetTransformatDistanceAlongSpline (Variables|Default|GetSpline) _output_get "Local" false))) (.y (.location (Spline|GetTransformatDistanceAlongSpline (Variables|Default|GetSpline) _output_get "Local" false))) (+ (.z (.location (Spline|GetTransformatDistanceAlongSpline (Variables|Default|GetSpline) _output_get "Local" false))) 1e+02)) (Math|Rotator|MakeRotator (.roll (.rotation (Spline|GetTransformatDistanceAlongSpline (Variables|Default|GetSpline) _output_get "Local" false))) (.pitch (.rotation (Spline|GetTransformatDistanceAlongSpline (Variables|Default|GetSpline) _output_get "Local" false))) (+ (.yaw (.rotation (Spline|GetTransformatDistanceAlongSpline (Variables|Default|GetSpline) _output_get "Local" false))) -9e+01)) "1.000000,1.000000,1.000000") false false)
      (Utilities|FlowControl|DelayUntilNextTick)
      (CallFunction|GotoRoom))))

(event Custom|ExitRoom
  (Variables|Default|SetMove true)
  (bind _output_get (Variables|Default|SetDistanceAlongSpline (+ (* (Utilities|Time|GetWorldDeltaSeconds) (Variables|Default|GetSplineSpeed)) (Variables|Default|GetDistanceAlongSpline))))
  (Transformation|SetRelativeTransform (Variables|Default|GetCapsule) (Math|Transform|MakeTransform (Math|Vector|MakeVector (.x (.location (Spline|GetTransformatDistanceAlongSpline (Variables|Default|GetSpline) _output_get "Local" false))) (.y (.location (Spline|GetTransformatDistanceAlongSpline (Variables|Default|GetSpline) _output_get "Local" false))) (+ (.z (.location (Spline|GetTransformatDistanceAlongSpline (Variables|Default|GetSpline) _output_get "Local" false))) 1e+02)) (Math|Rotator|MakeRotator (.roll (.rotation (Spline|GetTransformatDistanceAlongSpline (Variables|Default|GetSpline) _output_get "Local" false))) (.pitch (.rotation (Spline|GetTransformatDistanceAlongSpline (Variables|Default|GetSpline) _output_get "Local" false))) (+ (.yaw (.rotation (Spline|GetTransformatDistanceAlongSpline (Variables|Default|GetSpline) _output_get "Local" false))) -9e+01)) "1.000000,1.000000,1.000000") false false)
  (if (not (> (Variables|Default|GetDistanceAlongSpline) (Spline|GetSplineLength (Variables|Default|GetSpline))))
    (Utilities|FlowControl|DelayUntilNextTick)
    (CallFunction|ExitRoom)))

(event Custom|OnTextsEnd_Event
  (Variables|Default|SetTalking false)
  (CallFunction|ExitRoom)
  (Utilities|FlowControl|Delay 3.0)
  (Default|AddEmail (.AsWBP%20Monitor (Utilities|Casting|CastToWBP_Monitor (CallFunction|GetWidget "/Game/_CyberHexa/Blueprints/Widgets/WBP_Monitor.WBP_Monitor_C" false))) "Nie ma drugiego takiego jak ja – zatrudnij mnie!" "bobik.nolastname@klex.com" "Szanowni Państwo, 
 
Mam na imię Bobik i piszę do Was, bo wiem jedno: jestem najlepszym kandydatem na stanowisko, którego nawet jeszcze nie ogłosiliście. Ale kiedy ogłosicie – ja już tam będę. Gotowy. Z kawą. I pomysłami. 
 
Nie będę owijać w bawełnę – chcę pracować u Was bardzo. Tak bardzo, że już czuję się częścią zespołu. Serio. Nawet wymyśliłem sobie własne miejsce przy biurku. Jeśli będzie trzeba, przyniosę własne krzesło. Lub dwa. 
 
Wiem, że macie wielu kandydatów. Ale żaden z nich nie pisze tego maila teraz. Ja piszę. Bobik. Ten zdeterminowany. Ten z planem. Ten z ogromnym entuzjazmem, który można by sprzedawać w butelkach. 
 
Chętnie przyjdę, zadzwonię, połączę się przez Zooma, Teamsy, Skype’a, a nawet wyślę gołębia pocztowego, jeśli to skróci czas oczekiwania na spotkanie. 
 
W załączniku moje CV, choć i tak najwięcej mówią czyny – dlatego proszę o jedno: dajcie mi szansę pokazać, że warto. 
 
Czekam niecierpliwie na odpowiedź. A nawet niecierpliwiej niż to brzmi. 
 
Z motywacją większą niż espresso x3, 
Bobik"))

(event Custom|OnClicked_Event
  (params (TouchedActor :type Actor%20Object%20Reference) (ButtonPressed :type Key%20Structure :default "None")))

(event Custom|OnNextText_Event
  (params (Index :type Integer))
  (if (== Index 1)
    (Animation|Montage|PlayMontage (Variables|Default|GetSkeletalMesh) "/Game/_CyberHexa/Characters/AM_BobikGive.AM_BobikGive")))

(event Custom|OnBeginCursorOver_Event
  (params (TouchedActor :type Actor%20Object%20Reference)))

(event Custom|OnEndCursorOver_Event
  (params (TouchedActor :type Actor%20Object%20Reference)))

(event EventBeginPlay)

(fn ConstructionScript)