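; BP_Button is a player-triggered button that drives a character's visits to a room along the game mode's spline path.
; Box overlap starts the game mode's clock and, gated by a DoOnce that resets on exit, advances the spline state: enter room, leave, or bring in the next character.
; Each character's mesh, quote, montage and given item come from a DTJustMAilME row keyed by index and are pushed onto the spline path.
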(event OnComponentBeginOverlap(Box)
  (params (OverlappedComponent :type Primitive%20Component%20Object%20Reference) (OtherActor :type Actor%20Object%20Reference) (OtherComp :type Primitive%20Component%20Object%20Reference) (OtherBodyIndex :type Integer) (bFromSweep :type Boolean) (SweepResult :type Hit%20Result%20Structure%20%28by%20ref%29))
  (if (Actor|ActorHasTag OtherActor "player")
    (Variables|/Game/VRTemplate/Blueprints/VRGameMode.VRGameMode_C|SetClockStart (.AsVRGame%20Mode (Utilities|Casting|CastToVRGameMode (Game|GetGameMode))) true)
    (Utilities|FlowControl|DoOnce false
      (:Completed
        (switch Utilities|FlowControl|Switch|SwitchonE_SplineState (Variables|/Game/_CyberHexa/Blueprints/BP_SplinePath.BP_SplinePath_C|GetSplineState (Variables|Default|GetSpline%20Path))
          (:NewEnumerator0
            (Default|StartGotoRoom (Variables|Default|GetSpline%20Path)))
          (:NewEnumerator5
            (Default|StartExitRoom (Variables|Default|GetSpline%20Path)))
          (:NewEnumerator4
            (Math|Integer|IncrementInt (Variables|Default|GetSplineIndex)
              (:%20%20
                (CallFunction|ChangeCharacter (Variables|Default|GetSplineIndex))
                (Variables|/Game/_CyberHexa/Blueprints/BP_SplinePath.BP_SplinePath_C|SetSplineState (Variables|Default|GetSpline%20Path) "NewEnumerator0")
                (Default|StartGotoRoom (Variables|Default|GetSpline%20Path))))))))))

(event OnComponentEndOverlap(Box)
  (params (OverlappedComponent :type Primitive%20Component%20Object%20Reference) (OtherActor :type Actor%20Object%20Reference) (OtherComp :type Primitive%20Component%20Object%20Reference) (OtherBodyIndex :type Integer))
  (if (Actor|ActorHasTag OtherActor "player")
    (Utilities|FlowControl|DoOnce false) ; enters at Reset
  ))

(event Custom|ChangeCharacter
  (params (Index :type Integer))
  (bind _spline_path (Variables|Default|GetSpline%20Path))
  (bind _returnvalue (Utilities|GetDataTableRow (Variables|Default|GetDT_JustMAilME) (Utilities|String|StringToName (Utilities|String|ToString(Integer) Index)))
    (:then
      (Components|SkeletalMesh|SetSkeletalMeshAsset (Variables|/Game/_CyberHexa/Blueprints/BP_SplinePath.BP_SplinePath_C|GetSkeletalMesh _spline_path) (.Character (Utilities|Struct|BreakBS_JustMAilMe _returnvalue)))
      (Default|SetText (.AsWBP%20Character%20Quote (Utilities|Casting|CastToWBP_CharacterQuote (UserInterface|GetWidget (Variables|/Game/_CyberHexa/Blueprints/BP_SplinePath.BP_SplinePath_C|GetWidget _spline_path)))) (.Quote (Utilities|Struct|BreakBS_JustMAilMe _returnvalue)))
      (Variables|/Game/_CyberHexa/Blueprints/BP_SplinePath.BP_SplinePath_C|SetMontage%20to%20Play _spline_path (.Animation (Utilities|Struct|BreakBS_JustMAilMe _returnvalue)))
      (Variables|/Game/_CyberHexa/Blueprints/BP_SplinePath.BP_SplinePath_C|SetItem _spline_path (.GiveObject (Utilities|Struct|BreakBS_JustMAilMe _returnvalue))))))

(event Custom|TestStartOverlap
  (Utilities|FlowControl|DoOnce false
    (:Completed
      (switch Utilities|FlowControl|Switch|SwitchonE_SplineState (Variables|/Game/_CyberHexa/Blueprints/BP_SplinePath.BP_SplinePath_C|GetSplineState (Variables|Default|GetSpline%20Path))
        (:NewEnumerator0
          (Default|StartGotoRoom (Variables|Default|GetSpline%20Path)))
        (:NewEnumerator5
          (Default|StartExitRoom (Variables|Default|GetSpline%20Path)))
        (:NewEnumerator4
          (Math|Integer|IncrementInt (Variables|Default|GetSplineIndex)
            (:%20%20
              (CallFunction|ChangeCharacter (Variables|Default|GetSplineIndex))
              (Variables|/Game/_CyberHexa/Blueprints/BP_SplinePath.BP_SplinePath_C|SetSplineState (Variables|Default|GetSpline%20Path) "NewEnumerator0")
              (Default|StartGotoRoom (Variables|Default|GetSpline%20Path)))))))))

(event Custom|TestEndOverlap
  (Utilities|FlowControl|DoOnce false) ; enters at Reset
)

(event EventBeginPlay
  (Utilities|FlowControl|Delay 0.2)
  (Variables|Default|SetSpline%20Path (Variables|/Game/VRTemplate/Blueprints/VRGameMode.VRGameMode_C|GetBP_SplinePath (.AsVRGame%20Mode (Utilities|Casting|CastToVRGameMode (Game|GetGameMode)))))
  (CallFunction|ChangeCharacter 1))

(fn ConstructionScript)