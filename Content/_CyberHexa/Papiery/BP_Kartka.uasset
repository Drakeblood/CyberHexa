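; BP_Kartka is a clickable paper sheet that toggles between being attached to the camera pawn and resting in the world.
; Clicks alternate through a FlipFlop that sets the pawn's Ulotka (leaflet) flag, waits briefly, then attaches to the right bone socket keeping world transform.
; The next click clears the flag, detaches it and snaps the actor to a hardcoded location and rotation.
; The construction script applies the plane's material.
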(event Custom|OnClicked_Event
  (params (TouchedActor :type Actor%20Object%20Reference) (ButtonPressed :type Key%20Structure :default "None"))
  (Utilities|FlowControl|FlipFlop
    (:A
      (Variables|/Game/_CyberHexa/Blueprints/BP_CameraPawn.BP_CameraPawn_C|SetUlotka (CallFunction|GetCameraPawn) true)
      (Utilities|FlowControl|Delay 0.3)
      (Transformation|AttachComponentToComponent self (Variables|/Game/_CyberHexa/Blueprints/BP_CameraPawn.BP_CameraPawn_C|GetSkeletalMesh (CallFunction|GetCameraPawn)) "Socket_Bone_r" "KeepWorld" "KeepWorld" "KeepWorld" true))
    (:B
      (Variables|/Game/_CyberHexa/Blueprints/BP_CameraPawn.BP_CameraPawn_C|SetUlotka (CallFunction|GetCameraPawn) false)
      (Utilities|FlowControl|Delay 0.3)
      (Transformation|DetachFromComponent (Variables|Default|GetScene) "KeepWorld" "KeepWorld" "KeepWorld" true)
      (Transformation|SetActorLocationAndRotation "491.000000,-90.000000,560.000000" "0.000000,-99.999999,0.000000"))))

(event EventBeginPlay
  (EventDispatchers|BindEventtoOnClicked (delegate Custom|OnClicked_Event)))

(fn ConstructionScript
  (Rendering|Material|SetMaterial (Variables|Default|GetPlane) 0 (Variables|Default|GetMaterial)))