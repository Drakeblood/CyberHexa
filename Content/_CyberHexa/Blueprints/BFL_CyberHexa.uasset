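; BFL_CyberHexa is a Blueprint function library giving CyberHexa game code shortcuts to the camera pawn and UI widgets stored on GM_CyberHexa.
; GetWidget reuses the cached widget of a given class, or creates one for player 0 and caches it in the game mode's Widgets array.
; Showing a widget through GetWidget or ActivateWidget removes the current ActiveWidget from the viewport first, so these calls swap one active screen at a time.
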(fn GetCameraPawn
  (return (Variables|/Game/_CyberHexa/Blueprints/GM_CyberHexa.GM_CyberHexa_C|GetCameraPawn (.AsGM%20Cyber%20Hexa (Utilities|Casting|CastToGM_CyberHexa (Game|GetGameMode))))))

(fn GetWidget
  (params (WidgetClass :type User%20Widget%20Class%20Reference) (AddToViewport :type Boolean))
  (bind _array_element (Utilities|Array|ForEachLoopwithBreak (Variables|/Game/_CyberHexa/Blueprints/GM_CyberHexa.GM_CyberHexa_C|GetWidgets (.AsGM%20Cyber%20Hexa (Utilities|Casting|CastToGM_CyberHexa (Game|GetGameMode)))) :!label _label)
    (:LoopBody
      (if (== (Utilities|GetClass _array_element) WidgetClass)
        (LocalVariables|SetWidget _array_element)
        (goto _label Break)))
    (:Completed
      (LocalVariables|GetWidget
        (:then
          _)
        (:else
          (bind _returnvalue (UserInterface|CreateWidget WidgetClass (Game|GetPlayerController 0)))
          (bind _output_get (LocalVariables|SetWidget _returnvalue))
          (Utilities|Array|Add (Variables|/Game/_CyberHexa/Blueprints/GM_CyberHexa.GM_CyberHexa_C|GetWidgets (.AsGM%20Cyber%20Hexa (Utilities|Casting|CastToGM_CyberHexa (Game|GetGameMode)))) _output_get)))
      (if AddToViewport
        (bind _activewidget (Variables|/Game/_CyberHexa/Blueprints/GM_CyberHexa.GM_CyberHexa_C|GetActiveWidget (.AsGM%20Cyber%20Hexa (Utilities|Casting|CastToGM_CyberHexa (Game|GetGameMode))))
          (:then
            (Widget|RemovefromParent _activewidget))
          (:else
            _))
        (UserInterface|Viewport|AddtoViewport (LocalVariables|GetWidget) 0)
        (Variables|/Game/_CyberHexa/Blueprints/GM_CyberHexa.GM_CyberHexa_C|SetActiveWidget (.AsGM%20Cyber%20Hexa (Utilities|Casting|CastToGM_CyberHexa (Game|GetGameMode))) (LocalVariables|GetWidget)))
      (return (LocalVariables|GetWidget)))))

(fn RemoveActiveWidget
  (Widget|RemovefromParent (Variables|/Game/_CyberHexa/Blueprints/GM_CyberHexa.GM_CyberHexa_C|GetActiveWidget (.AsGM%20Cyber%20Hexa (Utilities|Casting|CastToGM_CyberHexa (Game|GetGameMode))))))

(fn ActivateWidget
  (params (Widget :type User%20Widget%20Object%20Reference))
  (CallFunction|RemoveActiveWidget)
  (UserInterface|Viewport|AddtoViewport Widget 0)
  (Variables|/Game/_CyberHexa/Blueprints/GM_CyberHexa.GM_CyberHexa_C|SetActiveWidget (.AsGM%20Cyber%20Hexa (Utilities|Casting|CastToGM_CyberHexa (Game|GetGameMode))) Widget))