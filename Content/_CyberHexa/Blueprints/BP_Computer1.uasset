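; BP_Computer1 is a clickable computer actor in CyberHexa that opens a monitor UI.
; On BeginPlay it registers itself with GM_CyberHexa and binds its click event.
; A click activates the existing WBP_Monitor widget, or creates and caches one on the viewport if none exists.
; A ChangeMaterial event lets the static mesh's first material slot be swapped.
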(event Custom|OnClicked_Event
  (params (TouchedActor :type Actor%20Object%20Reference) (ButtonPressed :type Key%20Structure :default "None"))
  (bind _monitorwidget (Variables|Default|GetMonitorWidget)
    (:then
      (CallFunction|ActivateWidget _monitorwidget))
    (:else
      (Variables|Default|SetMonitorWidget (.AsWBP%20Monitor (Utilities|Casting|CastToWBP_Monitor (CallFunction|GetWidget "/Game/_CyberHexa/Blueprints/Widgets/WBP_Monitor.WBP_Monitor_C" true)))))))

(event Custom|ChangeMaterial
  (params (Material :type Material%20Interface%20Object%20Reference))
  (Rendering|Material|SetMaterial (Variables|Default|GetStaticMesh) 0 Material))

(event EventBeginPlay
  (Variables|/Game/_CyberHexa/Blueprints/Framework/GM_CyberHexa.GM_CyberHexa_C|SetComputer (.AsGM%20Cyber%20Hexa (Utilities|Casting|CastToGM_CyberHexa (Game|GetGameMode))) self)
  (EventDispatchers|BindEventtoOnClicked (EventDispatchers|CreateEvent :!event Custom|OnClicked_Event)))

(fn ConstructionScript)