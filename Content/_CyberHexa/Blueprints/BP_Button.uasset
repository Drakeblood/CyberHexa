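; BP_Button is a player-triggered button that alternately sends a referenced spline path into and out of a room.
; A box overlap from an actor tagged "player" fires a DoOnce, which re-arms when that actor leaves.
; Each press runs a FlipFlop between GoToRoom and ExitRoom on the SplinePath.
; The cube is lowered, then its relative transform is reset immediately, with no delay.
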(event OnComponentBeginOverlap(Box)
  (params (OverlappedComponent :type Primitive%20Component%20Object%20Reference) (OtherActor :type Actor%20Object%20Reference) (OtherComp :type Primitive%20Component%20Object%20Reference) (OtherBodyIndex :type Integer) (bFromSweep :type Boolean) (SweepResult :type Hit%20Result%20Structure%20%28by%20ref%29))
  (bind _splinepath (CallFunction|GetSplinePath))
  (bind _cube (Variables|Default|GetCube))
  (if (Actor|ActorHasTag OtherActor "player")
    (Utilities|FlowControl|DoOnce false
      (:Completed
        (Transformation|SetRelativeLocation _cube "0.000000,0.000000,-20.000000" false false)
        (Transformation|ResetRelativeTransform _cube)
        (Utilities|FlowControl|FlipFlop
          (:A
            (Default|GotoRoom _splinepath))
          (:B
            (Default|ExitRoom _splinepath)))))))

(event OnComponentEndOverlap(Box)
  (params (OverlappedComponent :type Primitive%20Component%20Object%20Reference) (OtherActor :type Actor%20Object%20Reference) (OtherComp :type Primitive%20Component%20Object%20Reference) (OtherBodyIndex :type Integer))
  (bind _splinepath (CallFunction|GetSplinePath))
  (bind _cube (Variables|Default|GetCube))
  (if (Actor|ActorHasTag OtherActor "player")
    (Utilities|FlowControl|DoOnce false) ; enters at Reset
  ))

(event EventBeginPlay)

(event Collision|EventActorBeginOverlap
  (params (OtherActor :type Actor%20Object%20Reference)))

(event EventTick
  (params (DeltaSeconds :type Float%20%28single-precision%29)))

(fn ConstructionScript)